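; Master player character Blueprint handling camera-relative movement, look, jump, sprinting, aiming and an attached gun.
; The sprint axis sets a flag that switches the movement input scale and drives a timeline that animates camera FOV, reversing on release.
; The aim axis sets an aim flag and snaps FOV to a narrow value, with no explicit restore on release.
; BeginPlay spawns the gun and attaches it to the Vroid component's GunSocket.
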(event EventBeginPlay
  (bind _vroid (Variables|Default|GetVroid))
  ;[1 1 1] Gun
  (bind _returnvalue (Game|SpawnActorfromClass "/Game/Blueprints/BP_PlayerCharacters/BP-Master_Gun.BP-Master_Gun_C" (Transformation|GetWorldTransform _vroid) "Undefined" 0 0))
  (bind _output_get (Variables|Default|SetGun _returnvalue))
  (Transformation|AttachComponentToComponent _output_get _vroid "GunSocket" "SnapToTarget" "SnapToTarget" "SnapToTarget" true))

(event Input|ActionEvents|InputActionJump
  (params (Key :type Key%20Structure :default "None"))
  ;[1 1 1] Jump Logic
  (:Pressed
    (Character|Jump)))

(event Input|AxisEvents|InputAxisMoveFB
  (params (AxisValue :type Float%20%28single-precision%29))
  (bind _sprintmode (Variables|Default|GetSprintMode))
  ;[1 1 1] Movement Logic (w/ Sprint))
  (Math|Float|CompareFloat AxisValue 0.0
    (:>
      (if _sprintmode
        (Variables|Default|SetCurrentSpeed 1e+01)
        (else
          (Variables|Default|SetCurrentSpeed 0.5))))
    (:<
      (if _sprintmode
        (Variables|Default|SetCurrentSpeed -1e+01)
        (else
          (Variables|Default|SetCurrentSpeed -0.5)))))
  (Pawn|Input|AddMovementInput (Math|Vector|GetForwardVector (Transformation|GetWorldRotation (Variables|Default|GetCamera))) (Variables|Default|GetCurrentSpeed) false))

(event Input|AxisEvents|InputAxisMoveLR
  (params (AxisValue :type Float%20%28single-precision%29))
  (bind _sprintmode (Variables|Default|GetSprintMode))
  ;[1 1 1] Movement Logic (w/ Sprint))
  (Math|Float|CompareFloat AxisValue 0.0
    (:>
      (if _sprintmode
        (Variables|Default|SetCurrentSpeed 1e+01)
        (else
          (Variables|Default|SetCurrentSpeed 0.5))))
    (:<
      (if _sprintmode
        (Variables|Default|SetCurrentSpeed -1e+01)
        (else
          (Variables|Default|SetCurrentSpeed -0.5)))))
  (Pawn|Input|AddMovementInput (Math|Vector|GetRightVector (Transformation|GetWorldRotation (Variables|Default|GetCamera))) (Variables|Default|GetCurrentSpeed) false))

(event Input|AxisEvents|InputAxisLookLR
  (params (AxisValue :type Float%20%28single-precision%29))
  ;[1 1 1] Rotation Control
  (Pawn|Input|AddControllerYawInput AxisValue))

(event Input|AxisEvents|InputAxisLookUD
  (params (AxisValue :type Float%20%28single-precision%29))
  ;[1 1 1] Rotation Control
  (Pawn|Input|AddControllerPitchInput AxisValue))

(event Input|AxisEvents|InputAxisAim
  (params (AxisValue :type Float%20%28single-precision%29))
  (Math|Float|CompareFloat AxisValue 0.0
    (:>
      (Variables|Default|SetAim true)
      (bind _output_get (Variables|Default|SetAimSpeed 3e+01))
      (Camera|SetFieldOfView (Variables|Default|GetCamera) _output_get))
    (:==
      (Variables|Default|SetAim false :!label _label))
    (:<
      (goto _label))))

(event Input|AxisEvents|InputAxisSprintMode
  (params (AxisValue :type Float%20%28single-precision%29))
  ;[1 1 1] Sprint
  (Math|Float|CompareFloat AxisValue 0.0
    (:>
      (Variables|Default|SetSprintMode true)
      ;[1 1 1] SprintFOV
      (bind _tosprintfov (Timeline|SprintFOV Play)
        (:Update
          (Camera|SetFieldOfView (Variables|Default|GetCamera) _tosprintfov))))
    (:==
      (Variables|Default|SetSprintMode false :!label _label)
      (Timeline|SprintFOV Reverse))
    (:<
      (goto _label))))

(fn ConstructionScript)